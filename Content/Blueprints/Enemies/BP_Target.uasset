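; BP_Target is a damageable target actor in the enemies folder that dies when its health runs out.
; The construction script sets the Health component's value from an HP variable and binds to its dead delegate.
; AnyDamage forwards damage and its causer to the Health component, and OnDeadEvent turns on physics simulation for the target mesh.
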(event Custom|OnDeadEvent
  (Physics|SetSimulatePhysics (Variables|Default|GetTargetMesh) true))

(event Game|Damage|EventAnyDamage
  (params (Damage :type Float%20%28single-precision%29) (DamageType :type Damage%20Type%20Object%20Reference) (InstigatedBy :type Controller%20Object%20Reference) (DamageCauser :type Actor%20Object%20Reference))
  (Class|HealthComponent|ReceiveDamage (Variables|Default|GetHealth) Damage DamageCauser))

(fn ConstructionScript
  (EventDispatchers|BindEventtoDeadDelegate (Variables|Default|GetHealth) (EventDispatchers|CreateEvent :!event Custom|OnDeadEvent))
  (Variables|/Script/TestTask_JoyWay.HealthComponent|SetHealth (Variables|Default|GetHealth) (Variables|Default|GetHP)))