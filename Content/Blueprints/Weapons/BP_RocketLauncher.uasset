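; BP_RocketLauncher is a weapon Blueprint that adds rocket launcher feedback to a parent weapon class's fire and ready events.
; On fire it plays a reload sound, hides the Bullet component and plays a sped-up first-person fire montage on the owning BP_Player's FP mesh.
; When ready to fire again it unhides Bullet.
; The construction script assigns WeaponMesh as the parent's weapon mesh component.
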(event EventOnWeaponReadytoFire
  (|CallParentFunction)
  (Development|SetHiddeninGame (Variables|Default|GetBullet) false false))

(event EventOnWeaponFired
  (|CallParentFunction)
  (Components|Activation|Activate (Variables|Default|GetReloadAudio) true) ; Reloa sound every fire
  (Development|SetHiddeninGame (Variables|Default|GetBullet) true false)
  (bind _asbp_player (Utilities|Casting|CastToBP_Player (Components|GetOwner)))
  (Animation|Montage|PlayMontage (Variables|/Game/Blueprints/BP_Player.BP_Player_C|GetMeshFP _asbp_player) "/Game/FirstPerson/Animations/FirstPersonFire_Montage.FirstPersonFire_Montage" 1.5))

(fn ConstructionScript
  (Variables|Default|SetWeaponMeshComp (Variables|Default|GetWeaponMesh)))