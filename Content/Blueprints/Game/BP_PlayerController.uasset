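; Player controller that opens and closes the inventory screen.
; On BeginPlay it caches the BP_HUD, whose Inventory widget OpenInventory toggles in and out of the viewport.
; Showing it disables pawn input, shows the cursor and focuses the widget in Game and UI mode; hiding it restores game-only control.
; Both the Inventory input action and the CloseInventory event call this same toggle, so CloseInventory also opens a hidden inventory.
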(event EventCloseInventory
  (CallFunction|OpenInventory))

(event EventBeginPlay
  (bind _asbp_hud (Utilities|Casting|CastToBP_HUD (HUD|GetHUD)))
  (Variables|Default|SetHUD _asbp_hud))

(event Input|ActionEvents|InputActionInventory
  (params (Key :type Key%20Structure :default "None"))
  (:Pressed
    (CallFunction|OpenInventory)))

(fn ConstructionScript)

(fn OpenInventory
  (bind _returnvalue (Pawn|GetControlledPawn))
  (bind _hud (Variables|Default|GetHUD))
  (bind _inventory (Variables|/Game/Blueprints/Game/BP_HUD.BP_HUD_C|GetInventory _hud))
  (if (UserInterface|Viewport|IsinViewport (Variables|/Game/Blueprints/Game/BP_HUD.BP_HUD_C|GetInventory (Variables|Default|GetHUD)))
    (Widget|RemovefromParent _inventory)
    (Input|EnableInput _returnvalue 0)
    (Variables|Default|SetbShowMouseCursor false)
    (Input|SetInputModeGameOnly self)
    (else
      (UserInterface|Viewport|AddtoViewport _inventory 0)
      (Input|DisableInput _returnvalue 0)
      (Variables|Default|SetbShowMouseCursor true)
      (Input|SetInputModeGameandUI self (Variables|/Game/Blueprints/Game/BP_HUD.BP_HUD_C|GetInventory (Variables|Default|GetHUD)) "DoNotLock" false))))