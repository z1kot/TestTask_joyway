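; BP_DamageZone is an enemy hazard volume that repeatedly damages every actor inside its box.
; The construction script sets the actor tick interval to DamageRate, so Tick serves as the damage timer.
; Each tick, DamageAll applies Damage to all actors overlapping Box, with itself as causer, then re-activates the explosion particle.
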(event EventTick
  (params (DeltaSeconds :type Float%20%28single-precision%29))
  (CallFunction|DamageAll))

(fn ConstructionScript
  (Actor|Tick|SetActorTickInterval (Variables|Default|GetDamageRate)))

(fn DamageAll
  (for _array_element (Collision|GetOverlappingActors (Variables|Default|GetBox) "/Script/Engine.Actor" :!class /Script/Engine.PrimitiveComponent)
    (Game|Damage|ApplyDamage _array_element (Variables|Default|GetDamage) 0 self))
  (Components|Activation|Activate (Variables|Default|GetExplosionParticle) true))